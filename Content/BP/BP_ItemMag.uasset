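; BP_ItemMag is a magnet pickup item that calls Magnet on the Player who touches it.
; Overlap on the Sphere component triggers that call, plays a sound and destroys the item.
; Overlap on the Area component checks the player's Magnets flag and that it is player character 0.
; A timeline then pulls the item toward the player, adding its track value to a VInterpTo position on each update.
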(event `self.Sphere.OnComponentBeginOverlap`
  (params (OverlappedComponent :type "PrimitiveComponent Object Reference") (OtherActor :type "Actor Object Reference") (OtherComp :type "PrimitiveComponent Object Reference") (OtherBodyIndex :type Integer) (bFromSweep :type Boolean) (SweepResult :type "HitResult Structure (by ref)"))
  (bind _asplayer (cast `/Game/BP/Player` OtherActor))
  (`/Game/BP/Player.Magnet` _asplayer)
  (`GameplayStatics.PlaySoundAtLocation` "/Game/BGMSE/decision12.decision12" (`self.K2_GetActorLocation`) (struct) 1.0 1.0 0.0 null null null)
  (`self.K2_DestroyActor`))

(event `self.Area.OnComponentBeginOverlap`
  (params (OverlappedComponent :type "PrimitiveComponent Object Reference") (OtherActor :type "Actor Object Reference") (OtherComp :type "PrimitiveComponent Object Reference") (OtherBodyIndex :type Integer) (bFromSweep :type Boolean) (SweepResult :type "HitResult Structure (by ref)"))
  (bind _asplayer (cast `/Game/BP/Player` OtherActor))
  (if (`/Game/BP/Player.Magnets` _asplayer)
    (if (== OtherActor (`GameplayStatics.GetPlayerCharacter` 0))
      (bind (_direction `_新規track_0`) (`Timeline|タイムライン_0`)
        (:`Update`
          (`self.K2_SetActorLocation` (+ `_新規track_0` (`KismetMathLibrary.VInterpTo` (.location (`self.GetTransform`)) (`self.K2_GetActorLocation` (`GameplayStatics.GetPlayerCharacter` 0)) (`GameplayStatics.GetWorldDeltaSeconds`) 30.0))))))))

(fn `UserConstructionScript`)