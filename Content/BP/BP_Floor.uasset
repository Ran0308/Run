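; Endless-runner floor tile that asks MyGameMode to add another tile when the player overlaps its box, then destroys itself after a short delay.
; The construction script randomly fills it with a rock, coins or a magnet as child actors.
; Rocks and magnets use one of four spawn points, while coins scatter within CoinArea.
; GetAttachTransform exposes the AttachPoint world transform; the MagnetArea placement logic never runs.
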(event `self.Box.OnComponentBeginOverlap`
  (params (OverlappedComponent :type "PrimitiveComponent Object Reference") (OtherActor :type "Actor Object Reference") (OtherComp :type "PrimitiveComponent Object Reference") (OtherBodyIndex :type Integer) (bFromSweep :type Boolean) (SweepResult :type "HitResult Structure (by ref)"))
  (cast `/Game/BP/Player` OtherActor)
  (bind _asmy_game_mode (cast `/Game/BP/MyGameMode` (`GameplayStatics.GetGameMode`)))
  (`/Game/BP/MyGameMode.AddFloorTile` _asmy_game_mode)
  (`KismetSystemLibrary.Delay` 2.0)
  (`self.K2_DestroyActor`))

(fn `GetAttachTransform`
  (returns (ReturnValue :type "Transform Structure"))
  (return (`SceneComponent.K2_GetComponentToWorld` (`self.AttachPoint`))))

(fn `getSpawnPoints`
  (set `self.SpawnPoint` (`|MakeArray` (`SceneComponent.GetRelativeTransform` (`self.SpawnPoint1`)) (`SceneComponent.GetRelativeTransform` (`self.SpawnPoint2`)) (`SceneComponent.GetRelativeTransform` (`self.SpawnPoint3`)) (`SceneComponent.GetRelativeTransform` (`self.SpawnPoint4`)))))

(fn `SpawnCoins`
  (bind _coinarea (`self.CoinArea`))
  (for _ (range 11)
    (`AddComponent|NODE_AddChildActorComponent-2` :`RelativeTransform` (`KismetMathLibrary.Conv_VectorToTransform` (`KismetMathLibrary.RandomPointInBoundingBox` (`SceneComponent.RelativeLocation` _coinarea) (`BoxComponent.BoxExtent` _coinarea))))))

(fn `SpawnMagnet`
  (bind _spawnpoint (`self.SpawnPoint`))
  (`AddComponent|NODE_AddChildActorComponent-5` :`RelativeTransform` (`|GetArrayItem` _spawnpoint (`KismetMathLibrary.RandomIntegerInRange` 0 (`KismetArrayLibrary.Array_LastIndex` _spawnpoint)))))

(fn `SpawnRock`
  (bind _spawnpoint (`self.SpawnPoint`))
  (`AddComponent|NODE_AddChildActorComponent-0` :`RelativeTransform` (`|GetArrayItem` _spawnpoint (`KismetMathLibrary.RandomIntegerInRange` 0 (`KismetArrayLibrary.Array_LastIndex` _spawnpoint)))))

(fn `UserConstructionScript`
  (`self.getSpawnPoints`)
  (switch `int` (`KismetMathLibrary.RandomIntegerInRange` 0 2)
    (:`Default`
      (`self.SpawnRock` :!label _label))
    (:`0`
      (goto _label))
    (:`1`
      (`self.SpawnCoins`))
    (:`2`
      (`self.SpawnMagnet`))))