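; Coin pickup actor that homes in on the player and is collected on contact.
; Overlap of the Area component by player character 0 plays a timeline that moves the coin toward them each update, using VInterpTo plus the timeline track as an offset.
; Overlap of the Sphere component by a Player calls AddCoins on it, plays a money-drop sound and destroys the coin.
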(event `self.Sphere.OnComponentBeginOverlap`
  (params (OverlappedComponent :type "PrimitiveComponent Object Reference") (OtherActor :type "Actor Object Reference") (OtherComp :type "PrimitiveComponent Object Reference") (OtherBodyIndex :type Integer) (bFromSweep :type Boolean) (SweepResult :type "HitResult Structure (by ref)"))
  (bind _asplayer (cast `/Game/BP/Player` OtherActor))
  (`/Game/BP/Player.AddCoins` _asplayer)
  (`GameplayStatics.PlaySoundAtLocation` "/Game/BGMSE/money-drop1.money-drop1" (`self.K2_GetActorLocation`) (struct) 1.0 1.0 0.0 null null null)
  (`self.K2_DestroyActor`))

(event `self.Area.OnComponentBeginOverlap`
  (params (OverlappedComponent :type "PrimitiveComponent Object Reference") (OtherActor :type "Actor Object Reference") (OtherComp :type "PrimitiveComponent Object Reference") (OtherBodyIndex :type Integer) (bFromSweep :type Boolean) (SweepResult :type "HitResult Structure (by ref)"))
  (if true
    (if (== OtherActor (`GameplayStatics.GetPlayerCharacter` 0))
      (bind (_direction `_新規track_0`) (`Timeline|タイムライン_0`)
        (:`Update`
          (`self.K2_SetActorLocation` (+ `_新規track_0` (`KismetMathLibrary.VInterpTo` (.location (`self.GetTransform`)) (`self.K2_GetActorLocation` (`GameplayStatics.GetPlayerCharacter` 0)) (`GameplayStatics.GetWorldDeltaSeconds`) 15.0))))))))

(fn `UserConstructionScript`)